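; Spline actor that builds a chain of deformed meshes along its spline in the construction script, via the Wire function.
; SplineMeshVar selects the layout: one segment per pair of spline points using their tangents, or segments at Spacing intervals along the length.
; The spaced layout scales direction vectors by Spacing plus TangentScaleAdd for tangents.
; Every segment uses MainMesh with two material overrides.
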(fn ConstructionScript
  (|Wire))