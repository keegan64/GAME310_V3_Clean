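; BP_CCTV is a CCTV camera actor that captures the scene into a render target through a SceneCaptureComponent2D.
; On BeginPlay, CCTVID selects which of the four CCTV_CAM render targets the capture component writes to.
; EnableCCTV and DisableCCTV events switch per-frame capture on and off.
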(event Custom|EnableCCTV
  (Variables|/Script/Engine.SceneCaptureComponent|SetbCaptureEveryFrame (Variables|Default|GetSceneCaptureComponent2D) true))

(event Custom|DisableCCTV
  (Variables|/Script/Engine.SceneCaptureComponent|SetbCaptureEveryFrame (Variables|Default|GetSceneCaptureComponent2D) false))

(event EventBeginPlay
  (bind _scenecapturecomponent2d (Variables|Default|GetSceneCaptureComponent2D))
  (switch int (Variables|Default|GetCCTV_ID)
    (:0
      (Variables|/Script/Engine.SceneCaptureComponent2D|SetTextureTarget _scenecapturecomponent2d "/Game/CCTV_Assets/CCTV_CAM_1.CCTV_CAM_1"))
    (:1
      (Variables|/Script/Engine.SceneCaptureComponent2D|SetTextureTarget _scenecapturecomponent2d "/Game/CCTV_Assets/CCTV_CAM_2.CCTV_CAM_2"))
    (:2
      (Variables|/Script/Engine.SceneCaptureComponent2D|SetTextureTarget _scenecapturecomponent2d "/Game/CCTV_Assets/CCTV_CAM_3.CCTV_CAM_3"))
    (:3
      (Variables|/Script/Engine.SceneCaptureComponent2D|SetTextureTarget _scenecapturecomponent2d "/Game/CCTV_Assets/CCTV_CAM_4.CCTV_CAM_4"))))

(fn ConstructionScript)