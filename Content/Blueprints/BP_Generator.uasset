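; BP_Generator is a repairable generator actor that tells the first-person MetaHuman character when it is within interaction range.
; Entering InteractionBox registers the generator on the character and enables its use.
; Leaving resets the character's repair time, then either prints a cancel message for an unfinished repair or clears the reference and usage flags.
; The cancel branch leaves those flags set; repair progress and completion state live on the character.
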(event OnComponentBeginOverlap(InteractionBox)
  (params (OverlappedComponent :type Primitive%20Component%20Object%20Reference) (OtherActor :type Actor%20Object%20Reference) (OtherComp :type Primitive%20Component%20Object%20Reference) (OtherBodyIndex :type Integer) (bFromSweep :type Boolean) (SweepResult :type Hit%20Result%20Structure%20%28by%20ref%29))
  (bind _asbp_first_person_character_metahuman (Utilities|Casting|CastToBP_FirstPersonCharacter_Metahuman OtherActor))
  (Variables|/Game/FirstPerson/Blueprints/BP_FirstPersonCharacter_Metahuman.BP_FirstPersonCharacter_Metahuman_C|SetCurrentGenerator _asbp_first_person_character_metahuman self)
  (Variables|/Game/FirstPerson/Blueprints/BP_FirstPersonCharacter_Metahuman.BP_FirstPersonCharacter_Metahuman_C|SetCanUseGenerator _asbp_first_person_character_metahuman true))

(event OnComponentEndOverlap(InteractionBox)
  (params (OverlappedComponent :type Primitive%20Component%20Object%20Reference) (OtherActor :type Actor%20Object%20Reference) (OtherComp :type Primitive%20Component%20Object%20Reference) (OtherBodyIndex :type Integer))
  (bind _asbp_first_person_character_metahuman (Utilities|Casting|CastToBP_FirstPersonCharacter_Metahuman OtherActor))
  (Variables|/Game/FirstPerson/Blueprints/BP_FirstPersonCharacter_Metahuman.BP_FirstPersonCharacter_Metahuman_C|SetCurrentRepairTime _asbp_first_person_character_metahuman 0.0)
  (if (and (Variables|/Game/FirstPerson/Blueprints/BP_FirstPersonCharacter_Metahuman.BP_FirstPersonCharacter_Metahuman_C|GetIsRepairingGenerator _asbp_first_person_character_metahuman) (not (Variables|/Game/FirstPerson/Blueprints/BP_FirstPersonCharacter_Metahuman.BP_FirstPersonCharacter_Metahuman_C|GetHasRepairedGenerator _asbp_first_person_character_metahuman)))
    (Development|PrintString "Repair canceled")
    (else
      (Variables|/Game/FirstPerson/Blueprints/BP_FirstPersonCharacter_Metahuman.BP_FirstPersonCharacter_Metahuman_C|SetCurrentGenerator _asbp_first_person_character_metahuman 0)
      (Variables|/Game/FirstPerson/Blueprints/BP_FirstPersonCharacter_Metahuman.BP_FirstPersonCharacter_Metahuman_C|SetCanUseGenerator _asbp_first_person_character_metahuman false)
      (Variables|/Game/FirstPerson/Blueprints/BP_FirstPersonCharacter_Metahuman.BP_FirstPersonCharacter_Metahuman_C|SetIsRepairingGenerator _asbp_first_person_character_metahuman false))))

(event EventBeginPlay)

(event Collision|EventActorBeginOverlap
  (params (OtherActor :type Actor%20Object%20Reference)))

(event EventTick
  (params (DeltaSeconds :type Float%20%28single-precision%29)))

(fn ConstructionScript)