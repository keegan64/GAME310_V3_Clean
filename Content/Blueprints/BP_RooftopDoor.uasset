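; BP_RooftopDoor is the game-winning exit door, usable only while powered.
; Its InteractionBox overlaps toggle CanUseDoor and set or clear the Metahuman first-person character's CurrentDoor reference.
; UseDoor checks DoorPowered, then after a delay teleports the player to the TeleportLocation actor, shows WBP_Win and quits the game after another delay.
; CanUseDoor is not checked within this Blueprint.
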(event OnComponentBeginOverlap(InteractionBox)
  (params (OverlappedComponent :type Primitive%20Component%20Object%20Reference) (OtherActor :type Actor%20Object%20Reference) (OtherComp :type Primitive%20Component%20Object%20Reference) (OtherBodyIndex :type Integer) (bFromSweep :type Boolean) (SweepResult :type Hit%20Result%20Structure%20%28by%20ref%29))
  (Variables|Default|SetCanUseDoor true)
  (bind _asbp_first_person_character_metahuman (Utilities|Casting|CastToBP_FirstPersonCharacter_Metahuman OtherActor))
  (Variables|/Game/FirstPerson/Blueprints/BP_FirstPersonCharacter_Metahuman.BP_FirstPersonCharacter_Metahuman_C|SetCurrentDoor _asbp_first_person_character_metahuman self))

(event OnComponentEndOverlap(InteractionBox)
  (params (OverlappedComponent :type Primitive%20Component%20Object%20Reference) (OtherActor :type Actor%20Object%20Reference) (OtherComp :type Primitive%20Component%20Object%20Reference) (OtherBodyIndex :type Integer))
  (Variables|Default|SetCanUseDoor false)
  (bind _asbp_first_person_character_metahuman (Utilities|Casting|CastToBP_FirstPersonCharacter_Metahuman OtherActor))
  (Variables|/Game/FirstPerson/Blueprints/BP_FirstPersonCharacter_Metahuman.BP_FirstPersonCharacter_Metahuman_C|SetCurrentDoor _asbp_first_person_character_metahuman 0))

(event Custom|UseDoor
  (if (Variables|Default|GetDoorPowered)
    (Development|PrintString "Door Activated")
    (Utilities|FlowControl|Delay 2.0)
    (Transformation|SetActorLocation (Game|GetPlayerCharacter 0) (Transformation|GetActorLocation (Variables|Default|GetTeleportLocation)) false false)
    (bind _returnvalue (UserInterface|CreateWidget "/Game/UI/WBP_Win.WBP_Win_C"))
    (UserInterface|Viewport|AddtoViewport _returnvalue 0)
    (Utilities|FlowControl|Delay 5.0)
    (Game|QuitGame 0 "Quit" false)))

(event EventBeginPlay)

(event Collision|EventActorBeginOverlap
  (params (OtherActor :type Actor%20Object%20Reference)))

(event EventTick
  (params (DeltaSeconds :type Float%20%28single-precision%29)))

(fn ConstructionScript)