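; BP_ElevatorPanel is an interactable elevator panel that, once powered, teleports the player to a TeleportLocation actor.
; Its InteractionBox overlaps toggle CanUseElevator and register or clear the panel as the Metahuman first-person character's CurrentElevator.
; TurnOnPanel sets the powered flag and raises Emission on a dynamic material created at BeginPlay.
; UseElevator checks only that flag, prints a message, then moves player 0 after a short delay.
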(event OnComponentBeginOverlap(InteractionBox)
  (params (OverlappedComponent :type Primitive%20Component%20Object%20Reference) (OtherActor :type Actor%20Object%20Reference) (OtherComp :type Primitive%20Component%20Object%20Reference) (OtherBodyIndex :type Integer) (bFromSweep :type Boolean) (SweepResult :type Hit%20Result%20Structure%20%28by%20ref%29))
  (Variables|Default|SetCanUseElevator true)
  (bind _asbp_first_person_character_metahuman (Utilities|Casting|CastToBP_FirstPersonCharacter_Metahuman OtherActor))
  (Variables|/Game/FirstPerson/Blueprints/BP_FirstPersonCharacter_Metahuman.BP_FirstPersonCharacter_Metahuman_C|SetCurrentElevator _asbp_first_person_character_metahuman self))

(event OnComponentEndOverlap(InteractionBox)
  (params (OverlappedComponent :type Primitive%20Component%20Object%20Reference) (OtherActor :type Actor%20Object%20Reference) (OtherComp :type Primitive%20Component%20Object%20Reference) (OtherBodyIndex :type Integer))
  (Variables|Default|SetCanUseElevator false)
  (bind _asbp_first_person_character_metahuman (Utilities|Casting|CastToBP_FirstPersonCharacter_Metahuman OtherActor))
  (Variables|/Game/FirstPerson/Blueprints/BP_FirstPersonCharacter_Metahuman.BP_FirstPersonCharacter_Metahuman_C|SetCurrentElevator _asbp_first_person_character_metahuman 0))

(event Custom|TurnOnPanel
  (Rendering|Material|SetScalarParameterValue (Variables|Default|GetPanelMaterial) "Emission" 5e+01 :!class /Script/Engine.MaterialInstanceDynamic)
  (Rendering|Material|SetMaterial (Variables|Default|GetStaticMesh) 1 0)
  (Variables|Default|SetElevatorPowered true))

(event Custom|UseElevator
  (if (Variables|Default|GetElevatorPowered)
    (Development|PrintString "Elevator Activated")
    (Utilities|FlowControl|Delay 2.0)
    (Transformation|SetActorLocation (Game|GetPlayerCharacter 0) (Transformation|GetActorLocation (Variables|Default|GetTeleportLocation)) false false)))

(event Collision|EventActorBeginOverlap
  (params (OtherActor :type Actor%20Object%20Reference)))

(event EventTick
  (params (DeltaSeconds :type Float%20%28single-precision%29)))

(event EventBeginPlay
  (bind _returnvalue (Rendering|Material|CreateDynamicMaterialInstance (Variables|Default|GetStaticMesh) 2 0 "None" :!class /Script/Engine.PrimitiveComponent))
  (bind _output_get (Variables|Default|SetPanelMaterial _returnvalue))
  (Rendering|Material|SetScalarParameterValue _output_get "Emission" 0.0 :!class /Script/Engine.MaterialInstanceDynamic)
  (Rendering|Material|SetMaterial (Variables|Default|GetStaticMesh) 1 0))

(fn ConstructionScript)