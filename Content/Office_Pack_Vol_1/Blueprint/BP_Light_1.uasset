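; BP_Light_1 is an office lamp Blueprint that starts switched off and can be turned on.
; On BeginPlay it hides its three spotlights and creates a dynamic material instance on the lamp mesh with zero emission.
; The TurnOnLight event shows the spotlights and raises that material's Emission parameter so the lamp glows, with no matching turn-off event.
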(event Custom|TurnOnLight
  (Rendering|SetVisibility (Variables|Default|GetSpotLight) true false)
  (Rendering|SetVisibility (Variables|Default|GetSpotLight1) true false)
  (Rendering|SetVisibility (Variables|Default|GetSpotLight2) true false)
  (Rendering|Material|SetScalarParameterValue (Variables|Default|GetLightMaterial) "Emission" 1e+02 :!class /Script/Engine.MaterialInstanceDynamic))

(event Collision|EventActorBeginOverlap
  (params (OtherActor :type Actor%20Object%20Reference)))

(event EventTick
  (params (DeltaSeconds :type Float%20%28single-precision%29)))

(event EventBeginPlay
  (Rendering|SetVisibility (Variables|Default|GetSpotLight) false false)
  (Rendering|SetVisibility (Variables|Default|GetSpotLight1) false false)
  (Rendering|SetVisibility (Variables|Default|GetSpotLight2) false false)
  (bind _returnvalue (Rendering|Material|CreateDynamicMaterialInstance (Variables|Default|GetSM_lamp_2) 3 0 "None" :!class /Script/Engine.PrimitiveComponent))
  (Variables|Default|SetLightMaterial _returnvalue)
  (Rendering|Material|SetScalarParameterValue (Variables|Default|GetLightMaterial) "Emission" 0.0 :!class /Script/Engine.MaterialInstanceDynamic))

(fn ConstructionScript)